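; BP_UnderWater is an all-in-one underwater environment actor whose look is tuned through exposed variables.
; Its construction script pushes them into height fog with volumetric god rays, post process, skylight, sun and bounce lights, and the ocean surface mesh.
; It also assigns the Niagara dirt effect and passes itself to it as an object parameter, though the ParticleData event is empty.
; Fish visibility setters exist but are disconnected.
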(event EventParticleData
  (params (Data :type Array%20of%20Basic%20Particle%20Data%20Structures) (NiagaraSystem :type Niagara%20System%20Object%20Reference) (SimulationPositionOffset :type Vector%20%28by%20ref%29 :default "0, 0, 0")))

(fn ConstructionScript
  (bind _sunlight_bounced (Variables|Default|GetSunLight%20Bounced))
  (bind _color_grade_settings (Variables|PostProcess|GetColor%20Grade%20Settings))
  (bind _skylight (Variables|Default|GetSkyLight))
  (bind _directionallight (Variables|Default|GetDirectionalLight))
  (bind _sm_oceansurface (Variables|Default|GetSM_OceanSurface))
  (bind _p_dirt (Variables|Default|GetP_Dirt))
  (bind _exponentialheightfog (Variables|FogControls|GetExponentialHeightFog))
  (bind (_saturation _contrast _gamma _gain _offset) (Utilities|Struct|BreakColorGradePerRangeSettings _color_grade_settings))
  (Class|ExponentialHeightFogComponent|SetStartDistance _exponentialheightfog (Variables|FogControls|GetFog%20Distance))
  (Class|ExponentialHeightFogComponent|SetDirectionalInscatteringExponent _exponentialheightfog (Variables|FogControls|GetTop%20Surface%20Scattering))
  (Class|ExponentialHeightFogComponent|SetFogMaxOpacity _exponentialheightfog (Variables|FogControls|GetFog%20opacity))
  (Class|ExponentialHeightFogComponent|SetFogInscatteringColor _exponentialheightfog (Variables|FogControls|GetFog%20Colors))
  (Class|ExponentialHeightFogComponent|SetDirectionalInscatteringColor _exponentialheightfog (Variables|FogControls|GetTop%20surface%20Color))
  (Class|ExponentialHeightFogComponent|SetVolumetricFog _exponentialheightfog (Variables|volumetricFog|GetGodRays))
  (Class|ExponentialHeightFogComponent|SetVolumetricFogScatteringDistribution _exponentialheightfog (Variables|volumetricFog|GetGodRays%20Distribution%20))
  (Class|ExponentialHeightFogComponent|SetVolumetricFogExtinctionScale _exponentialheightfog (Variables|volumetricFog|GetGodRays%20Scale))
  (Class|ExponentialHeightFogComponent|SetVolumetricFogAlbedo _exponentialheightfog (Variables|volumetricFog|GetGodrays%20Albedo))
  (Class|ExponentialHeightFogComponent|SetVolumetricFogDistance _exponentialheightfog (Variables|volumetricFog|GetGodRays%20Distance))
  (Class|ExponentialHeightFogComponent|SetVolumetricFogEmissive _exponentialheightfog (Variables|volumetricFog|GetGodrays%20Emissive))
  (Utilities|Struct|SetmembersinPostProcessSettings (Variables|/Script/Engine.PostProcessComponent|GetSettings (Variables|PostProcess|GetPostProcess)) "BM_FFT" (Variables|PostProcess|GetTemp) (Variables|PostProcess|GetTint) _saturation _contrast _gamma _gain _offset (Variables|PostProcess|GetChromatic%20Intensity) (Variables|PostProcess|GetWater%20Blur) (Variables|PostProcess|GetReflection) (Variables|PostProcess|GetGlobal%20illumination) (Variables|PostProcess|GetExposure) (Variables|PostProcess|GetVignette%20Intensity) (Variables|PostProcess|GetPost%20Process%20Materials))
  (Rendering|Components|Light|SetIntensity _skylight (Variables|Lighting|GetHDRI%20Intensity))
  (Class|SkyLightComponent|SetCubemap _skylight (Variables|Lighting|Get%20Cubemap))
  (Rendering|Components|Light|SetLightColor _skylight (Variables|Lighting|GetHDRI%20Tint%20Color))
  (Rendering|Components|Light|SetIntensity _directionallight (Variables|Lighting|GetSunLight%20Intensity))
  (Rendering|Components|Light|SetLightColor _directionallight (Variables|Lighting|GetSunLight%20Color) true)
  (Class|DirectionalLightComponent|SetLightSourceSoftAngle _directionallight (Variables|Lighting|GetSunLight%20Soft%20Shadow))
  (Rendering|Components|Light|SetLightFunctionMaterial _directionallight (Variables|Lighting|GetLight%20Function%20Material))
  (Class|LightComponent|SetLightFunctionScale _directionallight (Variables|Lighting|GetLight%20Function%20Scale))
  (Class|LightComponent|SetVolumetricScatteringIntensity _directionallight (Variables|Lighting|Getvolumetric%20Light%20))
  (Class|LightComponentBase|SetCastVolumetricShadow _directionallight (Variables|Lighting|Getvolumetric%20Shadow))
  (Transformation|SetWorldTransform _sm_oceansurface (Variables|WaterSurface|Get%20Transform) false false)
  (Rendering|SetVisibility _sm_oceansurface (Variables|WaterSurface|GetWater%20Visibility) false)
  (Rendering|Material|SetMaterial _sm_oceansurface 0 (Variables|WaterSurface|GetMaterial))
  (Transformation|SetWorldTransform _directionallight (Variables|Lighting|GetSunLight%20Transform) false false)
  (Class|NiagaraComponent|SetAsset _p_dirt (Variables|Particles|GetNiagara) true)
  (Rendering|SetVisibility (Variables|Default|GetP_Dirt) (Variables|Particles|GetDirt%20Visibility) false)
  (Niagara|SetNiagaraVariable(Object) _p_dirt "" self)
  (Rendering|Components|Light|SetLightColor _sunlight_bounced (Variables|Lighting|GetSunLight%20Bounced%20Color) true)
  (Rendering|Components|Light|SetIntensity _sunlight_bounced (Variables|Lighting|GetSunLight%20Bounced%20Intensity)))